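; Zombie enemy that wanders randomly and chases and attacks the vampire player (BP_吸血鬼).
; A delayed AIMoveTo loop drives wandering until PawnSensing spots the vampire; reaching it triggers a DoOnce-gated attack montage, then wandering resumes.
; Right-hand overlaps, toggleable via 切換武器碰撞區域, deal random damage through the vampire's 受傷.
; Its own 受傷 subtracts health, halts movement and plays hurt or death montages, while Tick destroys it shortly after health runs out.
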(event OnComponentBeginOverlap(右手攻擊區域)
  (params (OverlappedComponent :type Primitive%20Component%20Object%20Reference) (OtherActor :type Actor%20Object%20Reference) (OtherComp :type Primitive%20Component%20Object%20Reference) (OtherBodyIndex :type Integer) (bFromSweep :type Boolean) (SweepResult :type Hit%20Result%20Structure%20%28by%20ref%29))
  ;[1 1 1] 攻擊回傳扣血
  (bind _asbp_吸血鬼 (Utilities|Casting|CastToBP_吸血鬼 OtherActor))
  (Default|受傷 _asbp_吸血鬼 (Math|Random|RandomFloatinRange 0.1 0.2)))

(event OnSeePawn(PawnSensing)
  (params (Pawn :type Pawn%20Object%20Reference))
  ;[1 1 1] 追蹤
  (if (not (Variables|Default|Get攻擊玩家)) ; 沒有攻擊才能追蹤
    (bind _asbp_吸血鬼 (Utilities|Casting|CastToBP_吸血鬼 Pawn))
    (bind _output_get (Variables|Default|Set吸血鬼物件 _asbp_吸血鬼))
    (AI|AIMoveTo self "0, 0, 0" _output_get 5.0 false
      (:OnSuccess
        (Utilities|FlowControl|DoOnce false :!label _label
          (:Completed
            (Animation|Montage|PlayMontage (Variables|Character|GetMesh) "/Game/動畫殭屍/殭屍攻擊_Montage.殭屍攻擊_Montage"
              (:then
                (Variables|Default|Set攻擊玩家 true)
                (Variables|Default|Set吸血鬼物件 0))
              (:OnCompleted
                (Variables|Default|Set攻擊玩家 false)
                (Utilities|FlowControl|Delay 0.5)
                (Utilities|FlowControl|Sequence
                  (:then_0
                    (goto _label Reset))
                  (:then_1
                    ;[1 1 1] 隨機走動
                    (if (not (Variables|Default|Get攻擊玩家)) :!label _label_2
                      (Utilities|IsValid (Variables|Default|Get吸血鬼物件)
                        (:Is%20Not%20Valid
                          (AI|AIMoveTo self (.RandomLocation (AI|Navigation|GetRandomReachablePointinRadius (Transformation|GetWorldLocation (Variables|Character|GetMesh)) 5e+02 0 0)) 0 5.0 false ; AI 前往指定位置
                            (:OnSuccess
                              (Utilities|FlowControl|Sequence
                                (:then_0
                                  _)))
                            (:OnFail
                              _))
                          (Utilities|FlowControl|Delay (Math|Random|RandomFloatinRange 1.0 3.5))
                          (goto _label_2))))))))))))))

(event Custom|受傷事件_Event
  ;[1 1 1] 受傷結束繼續走動追蹤
  (Variables|/Script/Engine.CharacterMovementComponent|SetMaxWalkSpeed (Variables|Character|GetCharacterMovement) 0.0)
  (Variables|Default|Set攻擊玩家 false)
  (Utilities|FlowControl|Sequence
    (:then_0
      ;[1 1 1] 隨機走動
      (AI|AIMoveTo self (.RandomLocation (AI|Navigation|GetRandomReachablePointinRadius (Transformation|GetWorldLocation (Variables|Character|GetMesh)) 5e+02 0 0)) 0 5.0 false :!label _label ; AI 前往指定位置
        (:OnSuccess
          (Utilities|FlowControl|Sequence
            (:then_0
              _)))
        (:OnFail
          _))
      (Utilities|FlowControl|Delay (Math|Random|RandomFloatinRange 1.0 3.5))
      (if (not (Variables|Default|Get攻擊玩家))
        (Utilities|IsValid (Variables|Default|Get吸血鬼物件)
          (:Is%20Not%20Valid
            (goto _label)))))
    (:then_1
      ;[1 1 1] 追蹤
      (Utilities|FlowControl|DoOnce false) ; enters at Reset
    )))

(event EventTick
  (params (DeltaSeconds :type Float%20%28single-precision%29))
  ;[1 1 1] 死亡
  (if (<= (Variables|Default|Get血量) 0.0)
    (Variables|Default|Set是否死亡 true)
    (Utilities|FlowControl|DoOnce false
      (:Completed
        (Utilities|FlowControl|Delay 3.0)
        (Actor|DestroyActor self)))))

(event EventBeginPlay
  ;[1 1 1] 隨機走動
  (Utilities|IsValid (Variables|Default|Get吸血鬼物件) :!label _label
    (:Is%20Not%20Valid
      (AI|AIMoveTo self (.RandomLocation (AI|Navigation|GetRandomReachablePointinRadius (Transformation|GetWorldLocation (Variables|Character|GetMesh)) 5e+02 0 0)) 0 5.0 false ; AI 前往指定位置
        (:OnSuccess
          (Utilities|FlowControl|Sequence
            (:then_0
              _)))
        (:OnFail
          _))
      (Utilities|FlowControl|Delay (Math|Random|RandomFloatinRange 1.0 3.5))
      (if (not (Variables|Default|Get攻擊玩家))
        (goto _label)))))

(fn ConstructionScript)

(fn 受傷
  (params (傷害值 :type Float%20%28single-precision%29))
  ;[1 1 1] 受傷
  (if (not (Variables|Default|Get是否死亡))
    (Variables|Default|Set血量 (- (Variables|Default|Get血量) 傷害值))
    (Animation|PlayAnimMontage self "/Game/動畫殭屍/殭屍受傷_Montage.殭屍受傷_Montage" 1.0 "None")
    (Variables|/Script/Engine.CharacterMovementComponent|SetMaxWalkSpeed (Variables|Character|GetCharacterMovement) 0.0)
    (if (<= (Variables|Default|Get血量) 0.0)
      (Animation|PlayAnimMontage self "/Game/動畫殭屍/殭屍死亡_Montage.殭屍死亡_Montage" 1.0 "None"))))

(fn 切換武器碰撞區域
  (params (是否顯示碰撞區域 :type Boolean))
  (Variables|/Script/Engine.PrimitiveComponent|SetbGenerateOverlapEvents (Variables|Default|Get右手攻擊區域) 是否顯示碰撞區域))